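; Game mode Blueprint that lays a chain of floor tiles when play begins.
; BeginPlay calls AddFloorTile in a short loop, spawning each FloorTile_BP at the attach transform of the previously spawned tile, tracked in LastSpawn.
; When no previous tile exists, the tile spawns at NextSpawnPoint.
; A delayed AddFloorTile call is present but never runs, and Tick is empty.
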(event `self.ReceiveBeginPlay`
  (for _ (range 5)
    (`self.AddFloorTile`)))

(event `self.ReceiveTick`
  (params (DeltaSeconds :type "Float (single-precision)")))

(fn `AddFloorTile`
  (bind _lastspawn (`self.LastSpawn`))
  (`/Engine/EditorBlueprintResources/StandardMacros.IsValid` _lastspawn
    (:`Is Valid`
      (bind _asfloor_tile_bp (cast `/Game/Blueprints/FloorTile_BP` _lastspawn))
      (bind _attachtransform (`/Game/Blueprints/FloorTile_BP.GetAttachTransform` _asfloor_tile_bp))
      (bind _returnvalue (`|SpawnActorFromClass` "/Game/Blueprints/FloorTile_BP.FloorTile_BP_C" _attachtransform "Undefined" "OverrideRootScale" null null))
      (set `self.LastSpawn` _returnvalue))
    (:`Is Not Valid`
      (bind _returnvalue_2 (`|SpawnActorFromClass` "/Game/Blueprints/FloorTile_BP.FloorTile_BP_C" (`self.NextSpawnPoint`) "Undefined" "OverrideRootScale" null null))
      (set `self.LastSpawn` _returnvalue_2))))

(fn `UserConstructionScript`)