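; Turtle enemy that advances along negative X to a stop line and periodically fires projectiles.
; Tick moves it a fixed, frame-rate-dependent step until it reaches the X position of the GameMode_BP EnemyStopArrow.
; A randomized timer starts on BeginPlay and calls FireBullets, which spawns a scaled-up EnemyProjectile_BP at BulletSpawn and re-arms itself with a longer random delay.
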(event `self.ReceiveBeginPlay`
  (`KismetSystemLibrary.K2_SetTimer` null "FireBullets" (`KismetMathLibrary.RandomFloatInRange` 3.0 4.0)))

(event `self.ReceiveTick`
  (params (DeltaSeconds :type "Float (single-precision)"))
  (bind (_returnvalue_x _returnvalue_y _returnvalue_z) (`KismetMathLibrary.BreakVector` (`self.K2_GetActorLocation`)))
  (bind _asgame_mode_bp (cast `/Game/Blueprints/GameMode_BP` (`GameplayStatics.GetGameMode`)))
  (bind _returnvalue_x_2 (`KismetMathLibrary.BreakVector` (`SceneComponent.K2_GetComponentLocation` (`/Game/Blueprints/GameMode_BP.EnemyStopArrow` _asgame_mode_bp))))
  (if (> _returnvalue_x _returnvalue_x_2)
    (`self.K2_SetActorLocation` (`KismetMathLibrary.MakeVector` (- _returnvalue_x 5.0) _returnvalue_y _returnvalue_z))))

(fn `FireBullets`
  (bind (_returnvalue_location _returnvalue_rotation) (`KismetMathLibrary.BreakTransform` (`SceneComponent.K2_GetComponentToWorld` (`self.BulletSpawn`))))
  (`|SpawnActorFromClass` "/Game/Blueprints/EnemyProjectile_BP.EnemyProjectile_BP_C" (`KismetMathLibrary.MakeTransform` _returnvalue_location _returnvalue_rotation (20.0 5.0 5.0)) "Undefined" "OverrideRootScale" null null)
  (`KismetSystemLibrary.K2_SetTimer` null "FireBullets" (`KismetMathLibrary.RandomFloatInRange` 5.0 6.0)))

(fn `UserConstructionScript`)