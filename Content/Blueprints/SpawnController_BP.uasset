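; SpawnController_BP periodically spawns random AI pawns (Enemy, Duck or Gecko) at arrow-marked points.
; The construction script caches three ahead and three behind arrow transforms.
; BeginPlay sets a looping SpawnEnemy timer on the first SpawnController found in the level, paced by SecondsPerEnemy.
; Chained random rolls pick the class, with Enemy and Duck spawning ahead and Gecko behind; location and rotation use separate random indices.
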(event `self.ReceiveBeginPlay`
  (bind _outactors (`GameplayStatics.GetAllActorsOfClass` "SpawnController_BP_C"))
  (bind _output_get (set `self.Spawner` (`|GetArrayItem` _outactors)))
  (`KismetSystemLibrary.K2_SetTimer` _output_get "SpawnEnemy" (/ (`self.SecondsPerEnemy`) 1.0) true))

(event `SpawnEnemy`
  (bind _returnvalue (`KismetMathLibrary.RandomIntegerInRange` 0 2))
  (bind _enemyspawnpointsbehind (`self.EnemySpawnPointsBehind`))
  (bind _enemyspawnpointsahead (`self.EnemySpawnPointsAhead`))
  (bind (_output_location _output_rotation) (`KismetMathLibrary.BreakTransform` (`|GetArrayItem` _enemyspawnpointsahead (`KismetMathLibrary.RandomIntegerInRange` 0 (`KismetArrayLibrary.Array_LastIndex` _enemyspawnpointsahead)))))
  (bind (_output_location_2 _output_rotation_2) (`KismetMathLibrary.BreakTransform` (`|GetArrayItem` _enemyspawnpointsbehind (`KismetMathLibrary.RandomIntegerInRange` 0 (`KismetArrayLibrary.Array_LastIndex` _enemyspawnpointsbehind)))))
  (if (== _returnvalue 0)
    (`AIBlueprintHelperLibrary.SpawnAIFromClass` "/Game/Blueprints/Enemy.Enemy_C" null _output_location _output_rotation)
    (elif (== _returnvalue 1)
      (`AIBlueprintHelperLibrary.SpawnAIFromClass` "/Game/Blueprints/Duck.Duck_C" null _output_location _output_rotation)
      (else
        (`AIBlueprintHelperLibrary.SpawnAIFromClass` "/Game/Blueprints/Gecko.Gecko_C" null _output_location_2 _output_rotation_2)))))

(fn `SetEnemySpawnPoints`
  (set `self.EnemySpawnPointsAhead` (`|MakeArray` (`SceneComponent.K2_GetComponentToWorld` (`self.SpawnAheadLArrow`)) (`SceneComponent.K2_GetComponentToWorld` (`self.SpawnAheadMArrow`)) (`SceneComponent.K2_GetComponentToWorld` (`self.SpawnAheadRArrow`))))
  (set `self.EnemySpawnPointsBehind` (`|MakeArray` (`SceneComponent.K2_GetComponentToWorld` (`self.SpawnBackLArrow`)) (`SceneComponent.K2_GetComponentToWorld` (`self.SpawnBackMArrow`)) (`SceneComponent.K2_GetComponentToWorld` (`self.SpawnBackRArrow`)))))

(fn `UserConstructionScript`
  (`self.SetEnemySpawnPoints`))