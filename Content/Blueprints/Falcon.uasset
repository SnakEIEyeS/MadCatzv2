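; Falcon is an actor, apparently an enemy, that flies toward a stop point defined by the game mode.
; Each Tick it casts the game mode to GameMode_BP and steps down world X while still beyond the EnemyStopArrow's X.
; The step is a fixed offset without delta-time scaling, so speed depends on frame rate.
; Disconnected leftover nodes hint at an abandoned direction-flag movement approach.
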(event `self.ReceiveBeginPlay`)

(event `self.ReceiveTick`
  (params (DeltaSeconds :type "Float (single-precision)"))
  (bind (_returnvalue_x _returnvalue_y _returnvalue_z) (`KismetMathLibrary.BreakVector` (`self.K2_GetActorLocation`)))
  (bind _asgame_mode_bp (cast `/Game/Blueprints/GameMode_BP` (`GameplayStatics.GetGameMode`)))
  (bind _returnvalue_x_2 (`KismetMathLibrary.BreakVector` (`SceneComponent.K2_GetComponentLocation` (`/Game/Blueprints/GameMode_BP.EnemyStopArrow` _asgame_mode_bp))))
  (if (> _returnvalue_x _returnvalue_x_2)
    (`self.K2_SetActorLocation` (`KismetMathLibrary.MakeVector` (- _returnvalue_x 10.0) _returnvalue_y _returnvalue_z))))

(fn `UserConstructionScript`)