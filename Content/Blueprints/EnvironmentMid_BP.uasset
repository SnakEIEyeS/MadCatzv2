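; EnvironmentMid_BP is a scrolling environment segment that endlessly chains copies of itself along the X axis.
; BeginPlay briefly spawns a FloorTile_BP to copy its TileMovingSpeed, then destroys it.
; Tick moves the root toward negative X by that speed without delta-time scaling, destroying the actor past DestroyXValue.
; The segment flagged LastPiece spawns its successor at SpawningPoint upon reaching SpawnNextXVal and passes the flag on.
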(event `self.ReceiveBeginPlay`
  ;[1 1 1] Begin play, get the floor tile speed
  (bind _returnvalue (`|SpawnActorFromClass` "/Game/Blueprints/FloorTile_BP.FloorTile_BP_C" (`KismetMathLibrary.MakeTransform` (-3000.0 0.0 0.0)) "Undefined" "OverrideRootScale" null null))
  (set `self.MovingSpeed` (`/Game/Blueprints/FloorTile_BP.TileMovingSpeed` _returnvalue))
  (`self.K2_DestroyActor` _returnvalue)
  (set `self.SpawningLocation` (`SceneComponent.K2_GetComponentLocation` (`self.SpawningPoint`))))

(event `self.ReceiveTick`
  (params (DeltaSeconds :type "Float (single-precision)"))
  (bind _defaultsceneroot (`self.DefaultSceneRoot`))
  (bind _returnvalue_x (`KismetMathLibrary.BreakVector` (`SceneComponent.K2_GetComponentLocation` _defaultsceneroot)))
  (bind _returnvalue (- _returnvalue_x (`self.MovingSpeed`)))
  (`SceneComponent.K2_SetWorldLocation` _defaultsceneroot (`KismetMathLibrary.MakeVector` _returnvalue) false false)
  (if (<= _returnvalue (`self.DestroyXValue`))
    (`self.K2_DestroyActor`)
    (elif (`self.LastPiece`)
      (if (<= _returnvalue (`self.SpawnNextXVal`))
        (`self.SpawnNextEnvironment`)))))

(event `SpawnNextEnvironment`
  ;[1 1 1] Spawning next environment tile
  (set `self.LastPiece` false)
  (bind _returnvalue (`|SpawnActorFromClass` "EnvironmentMid_BP_C" (`KismetMathLibrary.MakeTransform` (`SceneComponent.K2_GetComponentLocation` (`self.SpawningPoint`))) "Undefined" "OverrideRootScale" null null))
  (set `/Game/Blueprints/EnvironmentMid_BP.LastPiece` true _returnvalue))

(fn `UserConstructionScript`)