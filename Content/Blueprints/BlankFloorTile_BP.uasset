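; Blank floor tile that scrolls toward negative X to form a continuously extended track as the player progresses.
; Tick moves it a fixed step each frame, independent of delta time, and destroys it once it passes a rear X limit.
; When Character_BP overlaps EndTrigger, GameMode_BP is told to add another tile.
; GetAttachTransform exposes the AttachPoint's world transform.
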(event `self.ReceiveTick`
  (params (DeltaSeconds :type "Float (single-precision)"))
  (bind _returnvalue_x (`KismetMathLibrary.BreakVector` (`self.K2_GetActorLocation`)))
  (`self.K2_SetActorRelativeLocation` (`KismetMathLibrary.MakeVector` (- _returnvalue_x 5.0)))
  (if (< _returnvalue_x -3000.0)
    (`self.K2_DestroyActor`)))

(event `self.EndTrigger.OnComponentBeginOverlap`
  (params (OverlappedComponent :type "PrimitiveComponent Object Reference") (OtherActor :type "Actor Object Reference") (OtherComp :type "PrimitiveComponent Object Reference") (OtherBodyIndex :type Integer) (bFromSweep :type Boolean) (SweepResult :type "HitResult Structure (by ref)"))
  ;[1 1 1] Spawn and delete tiles as player progresses
  (cast `/Game/Blueprints/Character_BP` OtherActor)
  (bind _asgame_mode_bp (cast `/Game/Blueprints/GameMode_BP` (`GameplayStatics.GetGameMode`)))
  (`/Game/Blueprints/GameMode_BP.AddFloorTile` _asgame_mode_bp))

(fn `GetAttachTransform`
  (returns (AttachTransform :type "Transform Structure"))
  (return (`SceneComponent.K2_GetComponentToWorld` (`self.AttachPoint`))))

(fn `UserConstructionScript`)