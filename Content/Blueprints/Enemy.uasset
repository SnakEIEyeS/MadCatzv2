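; Enemy actor Blueprint that slides along the world X axis at a fixed step each frame.
; Tick offsets its location by a constant amount without delta time or sweep, so speed depends on frame rate.
; BeginPlay clears a MovementDir flag when spawned at positive X, but the movement ignores it.
; Disconnected nodes hint at unfinished direction switching and player-position logic.
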(event `self.ReceiveBeginPlay`
  (bind _returnvalue_x (`KismetMathLibrary.BreakVector` (`self.K2_GetActorLocation`)))
  (if (not (<= _returnvalue_x 0.0))
    (set `self.MovementDir` false)))

(event `self.ReceiveTick`
  (params (DeltaSeconds :type "Float (single-precision)"))
  (`self.K2_SetActorLocation` (+ (`self.K2_GetActorLocation`) (5.0 0.0 0.0))))

(fn `UserConstructionScript`)