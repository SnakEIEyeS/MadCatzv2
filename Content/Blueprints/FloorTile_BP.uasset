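; FloorTile_BP is a floor segment that recycles itself as the run progresses.
; Construction caches left, middle and right hazard point transforms, then adds a child actor hazard at a random one.
; When a Projectile_BP overlaps EndTrigger, the tile asks GameMode_BP to add a new tile, then destroys itself.
; GetAttachTransform exposes the AttachPoint's world transform.
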(event `self.ReceiveTick`
  (params (DeltaSeconds :type "Float (single-precision)")))

(event `self.EndTrigger.OnComponentBeginOverlap`
  (params (OverlappedComponent :type "PrimitiveComponent Object Reference") (OtherActor :type "Actor Object Reference") (OtherComp :type "PrimitiveComponent Object Reference") (OtherBodyIndex :type Integer) (bFromSweep :type Boolean) (SweepResult :type "HitResult Structure (by ref)"))
  ;[1 1 1] Spawn and delete tiles as player progresses
  (cast `/Game/Blueprints/Projectile_BP` OtherActor)
  (bind _asgame_mode_bp (cast `/Game/Blueprints/GameMode_BP` (`GameplayStatics.GetGameMode`)))
  (`/Game/Blueprints/GameMode_BP.AddFloorTile` _asgame_mode_bp)
  (`self.K2_DestroyActor`))

(fn `GetAttachTransform`
  (returns (AttachTransform :type "Transform Structure"))
  (return (`SceneComponent.K2_GetComponentToWorld` (`self.AttachPoint`))))

(fn `SetHazardPoints`
  (set `self.HazardPoints` (`|MakeArray` (`SceneComponent.GetRelativeTransform` (`self.HazardPointL`)) (`SceneComponent.GetRelativeTransform` (`self.HazardPointM`)) (`SceneComponent.GetRelativeTransform` (`self.HazardPointR`)))))

(fn `SpawnHazard`
  (bind _hazardpoints (`self.HazardPoints`))
  (`AddComponent|NODE_AddChildActorComponent-0` :`RelativeTransform` (`|GetArrayItem` _hazardpoints (`KismetMathLibrary.RandomIntegerInRange` 0 (`KismetArrayLibrary.Array_LastIndex` _hazardpoints)))))

(fn `UserConstructionScript`
  (`self.SetHazardPoints`)
  (`self.SpawnHazard`))